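; BP_CharacterBase is a base character that uses the Gameplay Ability System for sword melee combat.
; It acquires GA_Melee on BeginPlay and activates it through the MeleeAttack event.
; Sword collider overlaps with actors of exactly class BP_Enemy send a Skill.melee.dealdamage gameplay event to the character itself, with the enemy as target, and print the hit component.
; The Die event plays the Shinbi death montage.
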(event OnComponentBeginOverlap(SwordCollider)
  (params (OverlappedComponent :type Primitive%20Component%20Object%20Reference) (OtherActor :type Actor%20Object%20Reference) (OtherComp :type Primitive%20Component%20Object%20Reference) (OtherBodyIndex :type Integer) (bFromSweep :type Boolean) (SweepResult :type Hit%20Result%20Structure%20%28by%20ref%29))
  (if (!= OtherComp (Variables|Default|GetCapsuleComponent))
    (if (!= OtherActor self)
      (if (== (Utilities|GetClass OtherActor) "/Game/Blueprints/Characters/BP_Enemy.BP_Enemy_C")
        (Ability|SendGameplayEventtoActor self "(TagName=\"skill.melee.dealdamage\")" (Utilities|Struct|MakeGameplayEventData "" 0 OtherActor))
        (Development|PrintString (Utilities|GetDisplayName OtherComp))))))

(event Custom|MeleeAttack
  (Abilities|TryActivateAbilitybyClass (Variables|Default|GetAbilitySystemComp) "/Game/Blueprints/Characters/Abilities/Melee/GA_Melee.GA_Melee_C" true))

(event EventBeginPlay
  (Class|CharacterBase|AquireAbility "/Game/Blueprints/Characters/Abilities/Melee/GA_Melee.GA_Melee_C"))

(event Collision|EventActorBeginOverlap
  (params (OtherActor :type Actor%20Object%20Reference)))

(event EventTick
  (params (DeltaSeconds :type Float%20%28single-precision%29)))

(event EventDie
  (Animation|PlayAnimMontage "/Game/Blueprints/Characters/Animation/AM_Shinbi_Die.AM_Shinbi_Die" 1.0 "None"))

(fn ConstructionScript)